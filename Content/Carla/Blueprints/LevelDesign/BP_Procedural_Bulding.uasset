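; Procedural building actor that assembles a modular building from random mesh or Blueprint pieces, optionally at construction time.
; A moving transform cursor lays pieces along each side, stacking a base ring with doors, body floors with optional wall sides, a top ring and a roof grid.
; Meshes are batched into one HISM per mesh; Blueprint pieces become child actors whose first static mesh is hidden and instanced instead.
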(event EventBeginPlay)

(event Collision|EventActorBeginOverlap
  (params (OtherActor :type Actor%20Object%20Reference)))

(event EventTick
  (params (DeltaSeconds :type Float%20%28single-precision%29)))

(event EventDestroyed)

(fn ConstructionScript
  (if (Variables|Building|GetCreateAutomatically)
    (Building|CreateBuilding)))

(fn AddMeshtoBuilding
  (params (Mesh :type Static%20Mesh%20Object%20Reference) (Transform :type Transform))
  (bind _meshcomponent (Getters|GetMeshComponent Mesh))
  (Components|InstancedStaticMesh|AddInstance _meshcomponent Transform)
  (return _meshcomponent))

(fn GetMeshComponent
  (params (Mesh :type Static%20Mesh%20Object%20Reference))
  (bind _returnvalue (Utilities|GetObjectName Mesh))
  (bind _meshcomponentsmap (Variables|Default|GetMeshComponentsMap))
  (bind (_value _returnvalue_2) (Utilities|Map|Find _meshcomponentsmap _returnvalue))
  (if _returnvalue_2
    (return _value)
    (else
      (bind _returnvalue_3 (AddComponent|AddHierarchicalInstancedStaticMeshComponent false))
      (Components|StaticMesh|SetStaticMesh _returnvalue_3 Mesh)
      (Utilities|Map|Add (Variables|Default|GetMeshComponentsMap) _returnvalue _returnvalue_3)
      (return _returnvalue_3))))

(fn CreateRow
  (params (MainMeshes :type Array%20of%20Static%20Mesh%20Object%20References) (CornerMeshes :type Array%20of%20Static%20Mesh%20Object%20References) (MainBps :type Array%20of%20Actor%20Class%20References) (CornerBPs :type Array%20of%20Actor%20Class%20References) (Length :type Integer) (MainVisibility :type Boolean) (CornerVisibility :type Boolean))
  (if (or (> (Utilities|Array|Length MainMeshes) 0) (> (Utilities|Array|Length MainBps) 0))
    (for _index (range 0 (- Length 1))
      (bind (_mesh _bp) (Getters|GetActortoSpawn MainMeshes MainBps))
      (bind _z (Building|AddMesh _mesh _bp MainVisibility))
      (LocalVariables|SetZMax (Math|Float|Max(Float) _z (LocalVariables|GetZMax)))))
  (Utilities|FlowControl|Sequence
    (:then_0
      (if (and (Variables|Building|BaseParameters|GetCorners) (or (> (Utilities|Array|Length CornerMeshes) 0) (> (Utilities|Array|Length CornerBPs) 0)))
        (bind (_mesh_2 _bp_2) (Getters|GetActortoSpawn CornerMeshes CornerBPs))
        (bind (_z_2 _newparam) (Building|AddMesh _mesh_2 _bp_2 CornerVisibility))
        (LocalVariables|SetZMax (Math|Float|Max(Float) _z_2 (LocalVariables|GetZMax)))
        (Variables|Default|SetCurrentTransform (Math|Transform|MakeTransform (+ (.location (Variables|Default|GetCurrentTransform)) (* (Math|Vector|NegateVector (Math|Vector|GetRightVector (.rotation (Variables|Default|GetCurrentTransform)))) (.x (Utilities|GetMeshBounds _newparam)))) (.rotation (Variables|Default|GetCurrentTransform)) (.scale (Variables|Default|GetCurrentTransform))))))
    (:then_1
      (return (LocalVariables|GetZMax)))))

(fn CreateRing
  (params (MainMeshes :type Array%20of%20Static%20Mesh%20Object%20References) (CornerMeshes :type Array%20of%20Static%20Mesh%20Object%20References) (MainBps :type Array%20of%20Actor%20Class%20References) (CornerBPs :type Array%20of%20Actor%20Class%20References) (WallCheck :type Boolean))
  (for _index (range 0 (- (Utilities|Array|Length (Variables|Building|BaseParameters|GetSidesLength)) 1))
    (if WallCheck
      (if (and WallCheck (Utilities|Array|Get(acopy) (Variables|Building|BaseParameters|GetWalls) _index))
        (LocalVariables|SetMeshesOnRow (Variables|Building|Meshes|GetWallMeshes))
        (LocalVariables|SetBPsOnRow (Variables|Building|Meshes|GetWallBPs))
        (else
          (LocalVariables|SetMeshesOnRow MainMeshes :!label _label)
          (LocalVariables|SetBPsOnRow MainBps)))
      (else
        (goto _label)))
    (bind _maxz (Building|Generators|CreateRow (LocalVariables|GetMeshesOnRow) CornerMeshes (LocalVariables|GetBPsOnRow) CornerBPs (Utilities|Array|Get(acopy) (Variables|Building|BaseParameters|GetSidesLength) _index) (.SideVisibility (Utilities|ComputeVisibility _index)) (.CornerVisibility (Utilities|ComputeVisibility _index))))
    (LocalVariables|SetZMax (Math|Float|Max(Float) _maxz (LocalVariables|GetZMax)))
    (Utilities|UpdateFaceRotation))
  (Variables|Default|SetCurrentTransform (Math|Transform|MakeTransform (+ (.location (Variables|Default|GetCurrentTransform)) (Math|Vector|MakeVector 0.0 0.0 (LocalVariables|GetZMax))) (.rotation (Variables|Default|GetCurrentTransform)) (.scale (Variables|Default|GetCurrentTransform)))))

(fn CreateRingwithDoors
  (params (MainMeshes :type Array%20of%20Static%20Mesh%20Object%20References) (CornerMeshes :type Array%20of%20Static%20Mesh%20Object%20References) (MainBPs :type Array%20of%20Actor%20Class%20References) (CornerBPs :type Array%20of%20Actor%20Class%20References))
  (for _index (range 0 (- (Utilities|Array|Length (Variables|Building|BaseParameters|GetSidesLength)) 1))
    (bind _outset (Building|GetDoorsinRow (LocalVariables|GetBaseIndexDoorCounter) (Utilities|Array|Get(acopy) (Variables|Building|BaseParameters|GetSidesLength) _index)))
    (bind _maxz (Building|Generators|CreateRowwithDoors MainMeshes MainBPs CornerMeshes CornerBPs (Utilities|Array|Get(acopy) (Variables|Building|BaseParameters|GetSidesLength) _index) _outset (.SideVisibility (Utilities|ComputeVisibility _index)) (.CornerVisibility (Utilities|ComputeVisibility _index))))
    (LocalVariables|SetBaseIndexDoorCounter (+ (LocalVariables|GetBaseIndexDoorCounter) (Utilities|Array|Get(acopy) (Variables|Building|BaseParameters|GetSidesLength) _index)))
    (LocalVariables|SetZMax (Math|Float|Max(Float) _maxz (LocalVariables|GetZMax)))
    (Utilities|UpdateFaceRotation))
  (Variables|Default|SetCurrentTransform (Math|Transform|MakeTransform (+ (.location (Variables|Default|GetCurrentTransform)) (Math|Vector|MakeVector 0.0 0.0 (LocalVariables|GetZMax))) (.rotation (Variables|Default|GetCurrentTransform)) (.scale (Variables|Default|GetCurrentTransform)))))

(fn CreateRowwithDoors
  (params (MainMeshes :type Array%20of%20Static%20Mesh%20Object%20References) (MainBPs :type Array%20of%20Actor%20Class%20References) (CornerMeshes :type Array%20of%20Static%20Mesh%20Object%20References) (CornerBPs :type Array%20of%20Actor%20Class%20References) (Length :type Integer) (Doors :type Set%20of%20Integers) (MainVisibility :type Boolean) (CornerVisibility :type Boolean))
  (LocalVariables|SetprevTransform (Variables|Default|GetCurrentTransform))
  (if (or (> (Utilities|Array|Length MainMeshes) 0) (> (Utilities|Array|Length MainBPs) 0))
    (for _index (range 0 (- Length 1))
      (if (Utilities|Set|Contains Doors _index)
        (bind (_mesh _bp) (Getters|GetActortoSpawn (Variables|Building|Meshes|GetDoorMeshes) (Variables|Building|Meshes|GetDoorBPs)))
        (bind _z (Building|AddMesh _mesh _bp MainVisibility))
        (LocalVariables|SetZMax (Math|Float|Max(Float) _z (LocalVariables|GetZMax)))
        (else
          (bind (_mesh_2 _bp_2) (Getters|GetActortoSpawn MainMeshes MainBPs))
          (bind _z_2 (Building|AddMesh _mesh_2 _bp_2 MainVisibility))
          (LocalVariables|SetZMax (Math|Float|Max(Float) _z_2 (LocalVariables|GetZMax)))))))
  (Utilities|FlowControl|Sequence
    (:then_0
      (if (and (Variables|Building|BaseParameters|GetCorners) (or (> (Utilities|Array|Length CornerMeshes) 0) (> (Utilities|Array|Length CornerBPs) 0)))
        (bind (_mesh_3 _bp_3) (Getters|GetActortoSpawn CornerMeshes CornerBPs))
        (bind (_z_3 _newparam) (Building|AddMesh _mesh_3 _bp_3 MainVisibility))
        (LocalVariables|SetZMax (Math|Float|Max(Float) _z_3 (LocalVariables|GetZMax)))
        (Variables|Default|SetCurrentTransform (Math|Transform|MakeTransform (+ (.location (Variables|Default|GetCurrentTransform)) (* (Math|Vector|NegateVector (Math|Vector|GetRightVector (.rotation (Variables|Default|GetCurrentTransform)))) (.x (Utilities|GetMeshBounds _newparam)))) (.rotation (Variables|Default|GetCurrentTransform)) (.scale (Variables|Default|GetCurrentTransform))))))
    (:then_1
      (Utilities|Array|Add (Variables|Building|Debug|GetWallsStr) (* (+ (.location (Variables|Default|GetCurrentTransform)) (.location (LocalVariables|GetprevTransform)) (Math|Vector|MakeVector 0.0 0.0 (LocalVariables|GetZMax))) 0.5))
      (return (LocalVariables|GetZMax)))))

(fn GetDoorsinRow
  (params (MinIndex :type Integer) (Range :type Integer))
  (for _array_element (Variables|Building|BaseParameters|GetDoorsArray)
    (if (Math|Integer|InRange(Integer) _array_element MinIndex (+ MinIndex Range) true false)
      (Utilities|Set|Add (LocalVariables|GetOutputSet) (- _array_element MinIndex))))
  (return (LocalVariables|GetOutputSet)))

(fn CreateBuilding
  (Building|Reset)
  (Utilities|FlowControl|Sequence
    (:then_0
      (Building|Init))
    (:then_1
      (Building|Generators|CreateRingwithDoors (Variables|Building|Meshes|GetBaseMeshes) (Variables|Building|Meshes|GetCornerBaseMeshes) (Variables|Building|Meshes|GetBaseBPs) (Variables|Building|Meshes|GetCornerBaseBPs)))
    (:then_2
      (for _index (range 0 (- (Variables|Building|BaseParameters|GetNumFloors) 1))
        (Building|Generators|CreateRing (Variables|Building|Meshes|GetBodyMeshes) (Variables|Building|Meshes|GetCornerBodyMeshes) (Variables|Building|Meshes|GetBodyBPs) (Variables|Building|Meshes|GetCornerBodyBPs) (> (Utilities|Array|Length (Variables|Building|BaseParameters|GetWalls)) 0))))
    (:then_3
      (Building|Generators|CreateRing (Variables|Building|Meshes|GetTopMeshes) (Variables|Building|Meshes|GetCornerTopMeshes) (Variables|Building|Meshes|GetTopBPs) (Variables|Building|Meshes|GetCornerTopBPs) false)
      (Building|Generators|CreateRoof))))

(fn PrintState
  (bind _meshcomponentsmap (Variables|Default|GetMeshComponentsMap))
  (Utilities|FlowControl|Sequence
    (:then_0
      (bind _values (Utilities|Map|Values _meshcomponentsmap))
      (LocalVariables|SetDebugString (Utilities|String|Append "Num Instance Types: " (Utilities|String|ToString(Integer) (Utilities|Map|Length _meshcomponentsmap)) " - "))
      (for _array_element _values
        (LocalVariables|SetDebugString (Utilities|String|Append (LocalVariables|GetDebugString) (Utilities|String|ToString(Integer) (Components|InstancedStaticMesh|GetInstanceCount _array_element)) ", ")))
      (Development|PrintString (LocalVariables|GetDebugString) true true "(R=0.848958,G=0.690211,B=0.000000,A=1.000000)" 3.0))))

(fn Reset
  (bind _meshcomponentsmap (Variables|Default|GetMeshComponentsMap))
  (Utilities|FlowControl|Sequence
    (:then_0
      (bind _values (Utilities|Map|Values _meshcomponentsmap))
      (for _array_element _values
        (while (> (Components|InstancedStaticMesh|GetInstanceCount _array_element) 0)
          (Class|InstancedStaticMeshComponent|RemoveInstance _array_element)))
      (bind _keys (Utilities|Map|Keys _meshcomponentsmap))
      (for _array_element_2 _keys
        (Utilities|Map|Remove (Variables|Default|GetMeshComponentsMap) _array_element_2)))
    (:then_1
      (Variables|Default|SetCurrentTransform (Math|Transform|MakeTransform "0, 0, 0" "0,90.000000, 0" "1,1,1"))
      (Utilities|Array|Clear (Variables|Building|BaseParameters|GetDoorsArray))
      (Utilities|Array|Clear (Variables|Building|BaseParameters|GetSidesLength))
      (Utilities|Array|Clear (Variables|Building|Debug|GetWallsStr)))
    (:then_2
      (for _array_element_3 (Actor|GetAllChildActors true)
        (Actor|DestroyActor _array_element_3))
      (for _array_element_4 (Actor|GetComponentsByClass "/Script/Engine.ChildActorComponent")
        (Components|DestroyComponent _array_element_4)))))

(fn Init
  (bind _lengthx (Variables|Building|BaseParameters|GetLengthX))
  (bind _sideslength (Variables|Building|BaseParameters|GetSidesLength))
  (bind _lengthy (Variables|Building|BaseParameters|GetLengthY))
  (Utilities|FlowControl|Sequence
    (:then_0
      (if (Variables|Building|GetUseFullBlocks)
        (Utilities|Array|Add (Variables|Building|BaseParameters|GetSidesLength) 1)
        (else
          ;[1 1 1] Sides Length
          (Utilities|Array|Add _sideslength (Variables|Building|BaseParameters|GetLengthY))
          (Utilities|Array|Add _sideslength (Variables|Building|BaseParameters|GetLengthX))
          (Utilities|Array|Add _sideslength (Variables|Building|BaseParameters|GetLengthY))
          (Utilities|Array|Add _sideslength (Variables|Building|BaseParameters|GetLengthX)))))
    (:then_1
      ;[1 1 1] Doors
      (bind _result (Utilities|Set|ToArray (Variables|Building|BaseParameters|GetDoors)))
      (for _array_element _result
        (Utilities|Array|Add (Variables|Building|BaseParameters|GetDoorsArray) (Math|Integer|%(Integer) _array_element (+ _lengthx _lengthx _lengthy _lengthy)))))))

(fn Print3DState)

(fn CreateRoof
  (bind _cornertopmeshes (Variables|Building|Meshes|GetCornerTopMeshes))
  (Utilities|IsValid (Variables|Building|Meshes|GetRoofMesh)
    (:Is%20Valid
      (if (> (Utilities|Array|Length _cornertopmeshes) 0)
        (LocalVariables|SetInitalXOffset (.x (Utilities|GetMeshBounds (Utilities|Array|Get(acopy) _cornertopmeshes))))
        (else
          (LocalVariables|SetInitalXOffset (.x (Utilities|GetMeshBounds (Variables|Default|GetLastBPMeshAdded))))))
      (if (Variables|Building|BaseParameters|GetCorners)
        (Variables|Default|SetCurrentTransform (Math|Transform|MakeTransform (+ (Math|Vector|MakeVector (LocalVariables|GetInitalXOffset) 0.0 0.0) (.location (Variables|Default|GetCurrentTransform))) (.rotation (Variables|Default|GetCurrentTransform)) (.scale (Variables|Default|GetCurrentTransform)))))
      (for _index (range 0 (- (Variables|Building|BaseParameters|GetLengthX) 1))
        (LocalVariables|SettempLocation (.location (Variables|Default|GetCurrentTransform)))
        (for _index_2 (range 0 (- (Variables|Building|BaseParameters|GetLengthY) 1))
          (bind _newparam (Building|AddMesh (Variables|Building|Meshes|GetRoofMesh) 0 (Variables|Building|BaseParameters|Visibility|GetRoofVisibility))))
        (Variables|Default|SetCurrentTransform (Math|Transform|MakeTransform (+ (LocalVariables|GettempLocation) (* (Math|Vector|NegateVector (Math|Vector|GetRightVector (.rotation (Variables|Default|GetCurrentTransform)))) (.x (Utilities|GetMeshBounds _newparam)))) (.rotation (Variables|Default|GetCurrentTransform)) (.scale (Variables|Default|GetCurrentTransform))))))))

(fn GetActortoSpawn
  (params (Meshes :type Array%20of%20Static%20Mesh%20Object%20References) (BPs :type Array%20of%20Actor%20Class%20References))
  (bind _returnvalue (Utilities|Array|Length BPs))
  (bind _returnvalue_2 (Utilities|Array|Length Meshes))
  (if (and (> (Utilities|Array|Length Meshes) 0) (> (Utilities|Array|Length BPs) 0))
    (if (Math|Random|RandomBool)
      (LocalVariables|SetOutMesh (Utilities|Array|Get(acopy) Meshes (Math|Random|RandomInteger (Utilities|Array|Length Meshes))))
      (else
        (LocalVariables|SetOutBP (Utilities|Array|Get(acopy) BPs (Math|Random|RandomInteger (Utilities|Array|Length BPs))))))
    (return (LocalVariables|GetOutMesh) (LocalVariables|GetOutBP))
    (elif (> _returnvalue_2 0)
      (LocalVariables|SetOutMesh (Utilities|Array|Get(acopy) Meshes (Math|Random|RandomInteger _returnvalue_2)))
      (return (LocalVariables|GetOutMesh) (LocalVariables|GetOutBP))
      (elif (> _returnvalue 0)
        (LocalVariables|SetOutBP (Utilities|Array|Get(acopy) BPs (Math|Random|RandomInteger _returnvalue)))
        (return (LocalVariables|GetOutMesh) (LocalVariables|GetOutBP))))))

(fn AddMesh
  (params (Mesh :type Static%20Mesh%20Object%20Reference) (BP :type Actor%20Class%20Reference) (Visibility :type Boolean))
  (Utilities|IsValid Mesh
    (:Is%20Valid
      (LocalVariables|SetTempMesh Mesh)
      (if Visibility
        (Building|AddMeshtoBuilding (LocalVariables|GetTempMesh) (Variables|Default|GetCurrentTransform)))
      (Variables|Default|SetCurrentTransform (Math|Transform|MakeTransform (+ (.location (Variables|Default|GetCurrentTransform)) (* (* (Math|Vector|NegateVector (Math|Vector|GetForwardVector (.rotation (Variables|Default|GetCurrentTransform)))) (.x (Utilities|GetMeshBounds (LocalVariables|GetTempMesh)))) (Math|Conversions|ToInteger(Boolean) (not (Variables|Building|GetUseFullBlocks))))) (.rotation (Variables|Default|GetCurrentTransform)) (.scale (Variables|Default|GetCurrentTransform))))
      (return (.z (Utilities|GetMeshBounds (LocalVariables|GetTempMesh))) (LocalVariables|GetTempMesh)))
    (:Is%20Not%20Valid
      (if (Utilities|IsValidClass BP)
        (bind _returnvalue (AddComponent|AddChildActorComponent false (Variables|Default|GetCurrentTransform)))
        (ChildActorComponent|SetChildActorClass _returnvalue BP)
        (bind _output_get (LocalVariables|SetTempMesh (Variables|/Script/Engine.StaticMeshComponent|GetStaticMesh (Utilities|Array|Get(acopy) (Actor|GetComponentsByClass (Variables|/Script/Engine.ChildActorComponent|GetChildActor _returnvalue) "/Script/Engine.StaticMeshComponent")))))
        (if Visibility
          (Building|AddMeshtoBuilding _output_get (Variables|Default|GetCurrentTransform))
          (Rendering|SetVisibility (Utilities|Array|Get(acopy) (Actor|GetComponentsByClass (Variables|/Script/Engine.ChildActorComponent|GetChildActor _returnvalue) "/Script/Engine.StaticMeshComponent")) false false)
          (else
            (Components|DestroyComponent _returnvalue)))
        (Variables|Default|SetCurrentTransform (Math|Transform|MakeTransform (+ (.location (Variables|Default|GetCurrentTransform)) (* (* (Math|Vector|NegateVector (Math|Vector|GetForwardVector (.rotation (Variables|Default|GetCurrentTransform)))) (.x (Utilities|GetMeshBounds (LocalVariables|GetTempMesh)))) (Math|Conversions|ToInteger(Boolean) (not (Variables|Building|GetUseFullBlocks))))) (.rotation (Variables|Default|GetCurrentTransform)) (.scale (Variables|Default|GetCurrentTransform))))
        (Variables|Default|SetLastBPMeshAdded (LocalVariables|GetTempMesh))
        (return (.z (Utilities|GetMeshBounds (LocalVariables|GetTempMesh))) (LocalVariables|GetTempMesh))))))

(fn LockBuilding)