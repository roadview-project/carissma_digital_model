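; Winter tree generator that builds CARISSMA trees in the construction script, one static mesh component per DataTable row.
; Row locations are scaled by 100 and Y-flipped, with rotation and scale taken from the row.
; Chained SetTreeMesh calls match row-name substrings to tree types, then apply leaf and imposter materials by Season; spring materials and winter imposters are unassigned.
; An overlap-signature function forces the overlapped mesh to its highest-detail LOD.
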(fn ConstructionScript
  (bind _datatable (Variables|Default|GetDataTable))
  (bind _outrownames (DataTable|GetDataTableRowNames _datatable))
  (for _array_element _outrownames
    (bind _returnvalue (Utilities|GetDataTableRow _datatable _array_element)
      (:then
        (Utilities|FlowControl|Sequence
          (:then_0
            (bind _returnvalue_2 (AddComponent|AddStaticMeshComponent true (Math|Transform|MakeTransform (Math|Vector|MakeVector (.X (Math|Vector|BreakVector (* (.Location (Utilities|Struct|BreakTreeStruct _returnvalue)) 1e+02))) (* (.Y (Math|Vector|BreakVector (* (.Location (Utilities|Struct|BreakTreeStruct _returnvalue)) 1e+02))) -1.0) (.Z (Math|Vector|BreakVector (* (.Location (Utilities|Struct|BreakTreeStruct _returnvalue)) 1e+02)))) (.Rotation (Utilities|Struct|BreakTreeStruct _returnvalue)) (.Scale (Utilities|Struct|BreakTreeStruct _returnvalue)))))
            (Utilities|SetTreeMesh _returnvalue_2 "/Game/Carla/Static/Vegetation/CARISSMA/Single/Tree01_tree01.Tree01_tree01" (Utilities|String|ToString(Name) _array_element) "tree01" (Utilities|Struct|MakeTreeSeasonAssets "/Game/Carla/Static/Vegetation/CARISSMA/Single/CARISSMA_WinterTree01.CARISSMA_WinterTree01" "/Game/Carla/Static/Vegetation/CARISSMA/Textures/M_BranchFall.M_BranchFall" "/Game/Carla/Static/Vegetation/CARISSMA/ImposterTextures/Fall/MI_ImposterTree01_F.MI_ImposterTree01_F" "/Game/Carla/Static/Vegetation/CARISSMA/Textures/Branch1_material.Branch1_material") 1 2
              (:NotFound
                (Utilities|SetTreeMesh _returnvalue_2 "/Game/Carla/Static/Vegetation/CARISSMA/Single/Tree03_Autumn.Tree03_Autumn" (Utilities|String|ToString(Name) _array_element) "tree03" (Utilities|Struct|MakeTreeSeasonAssets "/Game/Carla/Static/Vegetation/CARISSMA/Single/CARISSMA_WinterTree03.CARISSMA_WinterTree03" "/Game/Carla/Static/Vegetation/CARISSMA/Textures/M_BranchFall.M_BranchFall" "/Game/Carla/Static/Vegetation/CARISSMA/ImposterTextures/Fall/MI_ImposterTree03_F.MI_ImposterTree03_F" "/Game/Carla/Static/Vegetation/CARISSMA/Textures/Branch1_material.Branch1_material") 1 2
                  (:NotFound
                    (Utilities|SetTreeMesh _returnvalue_2 "/Game/Carla/Static/Vegetation/CARISSMA/Single/TreeThin_Tree_thin.TreeThin_Tree_thin" (Utilities|String|ToString(Name) _array_element) "Tree_thin" (Utilities|Struct|MakeTreeSeasonAssets "/Game/Carla/Static/Vegetation/CARISSMA/Single/CARISSMA_TreeThin_Winter.CARISSMA_TreeThin_Winter" "/Game/Carla/Static/Vegetation/CARISSMA/Textures/M_BranchFall.M_BranchFall" "/Game/Carla/Static/Vegetation/CARISSMA/ImposterTextures/Fall/MI_ImposterThin_F.MI_ImposterThin_F" "/Game/Carla/Static/Vegetation/CARISSMA/Textures/Branch1_material.Branch1_material") 1 2
                      (:NotFound
                        (Utilities|SetTreeMesh _returnvalue_2 "/Game/Carla/Static/Vegetation/CARISSMA/Single/TreeSmall_Tree_small.TreeSmall_Tree_small" (Utilities|String|ToString(Name) _array_element) "Tree_small" (Utilities|Struct|MakeTreeSeasonAssets "/Game/Carla/Static/Vegetation/CARISSMA/Single/CARISSMA_TreeSmall_Winter.CARISSMA_TreeSmall_Winter" "/Game/Carla/Static/Vegetation/CARISSMA/Textures/M_BranchFall.M_BranchFall" "/Game/Carla/Static/Vegetation/CARISSMA/ImposterTextures/Fall/MI_ImposterTreeSmall_F.MI_ImposterTreeSmall_F" "/Game/Carla/Static/Vegetation/CARISSMA/Textures/Branch1_material.Branch1_material") 2 3
                          (:NotFound
                            (Utilities|SetTreeMesh _returnvalue_2 "/Game/Carla/Static/Vegetation/CARISSMA/Single/Tree02_Tree02.Tree02_Tree02" (Utilities|String|ToString(Name) _array_element) "Tree_large" (Utilities|Struct|MakeTreeSeasonAssets "/Game/Carla/Static/Vegetation/CARISSMA/Single/CARISSMA_Tree02_Winter.CARISSMA_Tree02_Winter" "/Game/Carla/Static/Vegetation/CARISSMA/Textures/M_BranchFall.M_BranchFall" "/Game/Carla/Static/Vegetation/CARISSMA/ImposterTextures/Fall/MI_ImposterTree02_F.MI_ImposterTree02_F" "/Game/Carla/Static/Vegetation/CARISSMA/Textures/Branch1_material.Branch1_material") 0 3
                              (:NotFound
                                (Utilities|SetTreeMesh _returnvalue_2 "/Game/Carla/Static/Vegetation/CARISSMA/Single/Tree_tree.Tree_tree" (Utilities|String|ToString(Name) _array_element) "tree_tree" (Utilities|Struct|MakeTreeSeasonAssets "/Game/Carla/Static/Vegetation/CARISSMA/Single/CARISSMA_WinterTree02.CARISSMA_WinterTree02" "/Game/Carla/Static/Vegetation/CARISSMA/Textures/M_BranchFall.M_BranchFall" "/Game/Carla/Static/Vegetation/CARISSMA/ImposterTextures/Fall/MI_ImposterTree_F.MI_ImposterTree_F" "/Game/Carla/Static/Vegetation/CARISSMA/Textures/Branch1_material.Branch1_material") 1 2)))))))))))))))))

(fn BPTreeGeneratorAutoGenFunc
  (params (OverlappedComponent :type Primitive%20Component%20Object%20Reference) (OtherActor :type Actor%20Object%20Reference) (OtherComp :type Primitive%20Component%20Object%20Reference) (OtherBodyIndex :type Integer) (bFromSweep :type Boolean) (SweepResult :type Hit%20Result%20Structure%20%28by%20ref%29))
  (bind _asstatic_mesh_component (Utilities|Casting|CastToStaticMeshComponent OverlappedComponent))
  (Rendering|LOD|SetForcedLodModel _asstatic_mesh_component 1))